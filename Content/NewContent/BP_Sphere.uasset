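; BP_Sphere is an actor that moves in a straight line and bounces off whatever it hits, gradually losing speed.
; Each Tick it applies a swept world offset from Direction and Speed scaled by delta time.
; On a blocking hit it reflects Direction about the surface normal, cuts Speed by a tenth, prints it, and stops entirely once Speed falls to MinSpeed or below.
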(event EventBeginPlay)

(event Collision|EventActorBeginOverlap
  (params (OtherActor :type Actor%20Object%20Reference)))

(event EventTick
  (params (DeltaSeconds :type Float%20%28single-precision%29))
  (bind _sweephitresult (Transformation|AddActorWorldOffset (* (* (Variables|Default|GetDirection) (Variables|Default|Getspeed)) DeltaSeconds) true))
  (if (.bBlockingHit (Collision|BreakHitResult _sweephitresult))
    (Variables|Default|SetDirection (Math|Vector|GetReflectionVector (Variables|Default|GetDirection) (.Normal (Collision|BreakHitResult _sweephitresult))))
    (bind _output_get (Variables|Default|Setspeed (- (Variables|Default|Getspeed) (* (Variables|Default|Getspeed) 0.1))))
    (Development|PrintString (Utilities|String|ToString(Float) (Variables|Default|Getspeed)))
    (if (>= (Variables|Default|GetMin%20speed) _output_get)
      (Variables|Default|Setspeed 0.0))))

(fn ConstructionScript)